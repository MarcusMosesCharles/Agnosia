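; BPC_Wraiths is a wraith character that uses AI movement to pursue the player.
; Every Tick issues a new AIMoveTo targeting player controller 0, rather than the player pawn.
; A separate IgnoreActors event, not called within this graph, makes the mesh and capsule ignore all BP_Door actors and the player pawn when moving, so neither blocks the wraith.
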(event `self.ReceiveBeginPlay`)

(event `self.ReceiveTick`
  (params (DeltaSeconds :type "Float (single-precision)"))
  (`|AIMoveTo` self (0.0 0.0 0.0) (`GameplayStatics.GetPlayerController` 0)))

(event `IgnoreActors`
  (bind _returnvalue (`GameplayStatics.GetPlayerPawn` 0))
  (bind _outactors (`GameplayStatics.GetAllActorsOfClass` "/Game/_Content/_SceneActors/BP_Door.BP_Door_C"))
  (for _array_element _outactors
    (`PrimitiveComponent.IgnoreActorWhenMoving` (`self.Mesh`) _array_element true))
  (for _array_element_2 _outactors
    (`PrimitiveComponent.IgnoreActorWhenMoving` (`self.CapsuleComponent`) _array_element_2 true))
  (`PrimitiveComponent.IgnoreActorWhenMoving` (`self.Mesh`) _returnvalue true)
  (`PrimitiveComponent.IgnoreActorWhenMoving` (`self.CapsuleComponent`) _returnvalue true))

(fn `UserConstructionScript`)