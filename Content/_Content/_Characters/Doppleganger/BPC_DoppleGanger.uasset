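; Doppelganger monster character that flickers in and out of view, laughs periodically and jumpscares the player on contact.
; Sphere overlap, pawn sensing and the VisionwireNaming function set the AI blackboard's PlayerDetected key, which an outer sphere exit clears; VisionwireNaming also briefly glitches the player's screen.
; A capsule hit teleports the player, switches the view to the monster, then relocates it to a random Doppelganger point and restores the view with fades.
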(event `self.ReceiveTick`
  (params (DeltaSeconds :type "Float (single-precision)"))
  (`self.Laughter`)
  (`self.Visibility`))

(event `Laughter`
  (`KismetSystemLibrary.Delay` (`KismetMathLibrary.RandomFloatInRange` 4.0 6.0))
  (`GameplayStatics.PlaySoundAtLocation` "/Game/_Content/_Audio/SC_Laugh.SC_Laugh" (`self.K2_GetActorLocation`) (struct) 1.0 1.0 0.0 null null null null))

(event `Visibility`
  (bind _returnvalue (`KismetMathLibrary.RandomFloatInRange` 0.1 0.5))
  (bind _groom (`self.Groom`))
  (bind _mesh (`self.Mesh`))
  (if (`self.WarpToggle`)
    (if (`self.Warping`)
      (`SceneComponent.SetVisibility` _groom true false)
      (`SceneComponent.SetVisibility` _mesh true false)
      (`KismetSystemLibrary.Delay` _returnvalue)
      (set `self.Warping` false)
      (else
        (`SceneComponent.SetVisibility` _groom false false)
        (`SceneComponent.SetVisibility` _mesh false false)
        (`KismetSystemLibrary.Delay` _returnvalue)
        (set `self.Warping` true)))))

(event `Glitch`
  (bind _asbp_first_person_character (cast `/Game/FirstPerson/Blueprints/BP_FirstPersonCharacter` (`GameplayStatics.GetPlayerPawn` 0)))
  (set `/Game/FirstPerson/Blueprints/BP_FirstPersonCharacter.GlitchIntensity` 2 _asbp_first_person_character)
  (`KismetSystemLibrary.Delay` 2.0)
  (set `/Game/FirstPerson/Blueprints/BP_FirstPersonCharacter.GlitchIntensity` 0 _asbp_first_person_character))

(event `self.Sphere.OnComponentBeginOverlap`
  (params (OverlappedComponent :type "PrimitiveComponent Object Reference") (OtherActor :type "Actor Object Reference") (OtherComp :type "PrimitiveComponent Object Reference") (OtherBodyIndex :type Integer) (bFromSweep :type Boolean) (SweepResult :type "HitResult Structure (by ref)"))
  (cast `/Game/FirstPerson/Blueprints/BP_FirstPersonCharacter` OtherActor)
  (`BlackboardComponent.SetValueAsBool` (`AIBlueprintHelperLibrary.GetBlackboard` (`AIBlueprintHelperLibrary.GetAIController` self)) "PlayerDetected" true :!label _label))

(event `self.PawnSensing.OnSeePawn`
  (params (Pawn :type "Pawn Object Reference"))
  (cast `/Game/FirstPerson/Blueprints/BP_FirstPersonCharacter` Pawn)
  (goto _label))

(event `self.Sphere1.OnComponentEndOverlap`
  (params (OverlappedComponent :type "PrimitiveComponent Object Reference") (OtherActor :type "Actor Object Reference") (OtherComp :type "PrimitiveComponent Object Reference") (OtherBodyIndex :type Integer))
  (cast `/Game/FirstPerson/Blueprints/BP_FirstPersonCharacter` OtherActor)
  (`BlackboardComponent.SetValueAsBool` (`AIBlueprintHelperLibrary.GetBlackboard` (`AIBlueprintHelperLibrary.GetAIController` self)) "PlayerDetected" false)
  (set `CharacterMovementComponent.MaxWalkSpeed` 150.0 (`self.CharacterMovement`)))

(event `self.CapsuleComponent.OnComponentHit`
  (params (HitComponent :type "PrimitiveComponent Object Reference") (OtherActor :type "Actor Object Reference") (OtherComp :type "PrimitiveComponent Object Reference") (NormalImpulse :type "Vector Structure") (Hit :type "HitResult Structure (by ref)"))
  (bind _returnvalue (`GameplayStatics.GetPlayerCameraManager` 0))
  (cast `/Game/FirstPerson/Blueprints/BP_FirstPersonCharacter` OtherActor)
  (bind _returnvalue_2 (`GameplayStatics.GetActorOfClass` "/Game/_Content/_SceneActors/NewPosition.NewPosition_C"))
  (`self.K2_SetActorRelativeTransform` (`GameplayStatics.GetPlayerPawn` 0) (`self.GetTransform` _returnvalue_2) false true)
  (bind _outactors (`GameplayStatics.GetAllActorsOfClass` "/Game/_Content/_Characters/Doppleganger/Blueprints/BP_DOpplegangerPoints.BP_DOpplegangerPoints_C"))
  (`self.Jumpscare`)
  (`KismetSystemLibrary.Delay` 0.8)
  (`self.K2_SetActorRelativeTransform` (`self.GetTransform` (`KismetArrayLibrary.Array_Random` _outactors)) false true)
  (bind _returnvalue_3 (`GameplayStatics.GetActorOfClass` "/Game/FirstPerson/Blueprints/BP_FirstPersonCharacter.BP_FirstPersonCharacter_C"))
  (`PlayerCameraManager.StartCameraFade` :`self` _returnvalue :`ToAlpha` 1.0 :`Duration` 1.0)
  (`PlayerController.SetViewTargetWithBlend` (`GameplayStatics.GetPlayerController` 0) _returnvalue_3 0.0 "VTBlend_Linear" 0.0 false)
  (set `CharacterMovementComponent.MaxWalkSpeed` 150.0 (`self.CharacterMovement`))
  (set `self.WarpToggle` true)
  (set `self.JumpscareTriggered` false)
  (`PlayerCameraManager.StartCameraFade` :`self` _returnvalue :`FromAlpha` 1.0 :`ToAlpha` 0.0 :`Duration` 0.5))

(event `Jumpscare`
  (`PlayerController.SetViewTargetWithBlend` (`GameplayStatics.GetPlayerController` 0) self 0.0 "VTBlend_Linear" 0.0 false)
  (set `CharacterMovementComponent.MaxWalkSpeed` 0.0 (`self.CharacterMovement`))
  (set `self.WarpToggle` false)
  (`SceneComponent.SetVisibility` (`self.Mesh`) true false)
  (set `self.JumpscareTriggered` true)
  (`GameplayStatics.PlaySound2D` "/Game/_Content/_Audio/Jumpscare/SC_Jumspcare.SC_Jumspcare" 1.0 1.0 0.0 null null))

(fn `UserConstructionScript`)

(fn `VisionwireNaming`
  (returns (Name :type String) (IsMonster :type Boolean))
  (`BlackboardComponent.SetValueAsBool` (`AIBlueprintHelperLibrary.GetBlackboard` (`AIBlueprintHelperLibrary.GetAIController` self)) "PlayerDetected" true)
  (`self.Glitch`)
  (return "Monster" true))