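; Doppleganger stalker that peeks at the player and vanishes when seen or approached.
; VisionwireNaming triggers SeenbyPlayer, which plays the peek-hide animation once, then destroys the actor after a delay.
; Player overlap with its box plays a laugh at the BP_DoorTeleport location, destroys the actor and raises the player's GlitchIntensity.
; The glitch reset follows a Delay placed after DestroyActor.
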(event `Seen by Player`
  (`/Engine/EditorBlueprintResources/StandardMacros.DoOnce` false
    (:`Completed`
      (`SkeletalMeshComponent.PlayAnimation` (`self.SkeletalMesh`) "/Game/_Content/_Characters/Doppleganger/Temp/DoppleGangerAnimations_Anim_A_Peaking_Hide.DoppleGangerAnimations_Anim_A_Peaking_Hide" false)
      (`KismetSystemLibrary.Delay` 1.0)
      (`self.K2_DestroyActor`))))

(event `self.Box.OnComponentBeginOverlap`
  (params (OverlappedComponent :type "PrimitiveComponent Object Reference") (OtherActor :type "Actor Object Reference") (OtherComp :type "PrimitiveComponent Object Reference") (OtherBodyIndex :type Integer) (bFromSweep :type Boolean) (SweepResult :type "HitResult Structure (by ref)"))
  (bind _asbp_first_person_character (cast `/Game/FirstPerson/Blueprints/BP_FirstPersonCharacter` OtherActor))
  (bind _returnvalue (`GameplayStatics.GetActorOfClass` "/Game/_Content/_SceneActors/BP_DoorTeleport.BP_DoorTeleport_C"))
  (`GameplayStatics.PlaySoundAtLocation` "/Game/_Content/_Audio/SC_Laugh.SC_Laugh" (`self.K2_GetActorLocation` _returnvalue) (struct) 1.0 1.0 0.0 null null null null)
  (`self.K2_DestroyActor`)
  (set `/Game/FirstPerson/Blueprints/BP_FirstPersonCharacter.GlitchIntensity` 2 _asbp_first_person_character)
  (`KismetSystemLibrary.Delay` 0.5)
  (set `/Game/FirstPerson/Blueprints/BP_FirstPersonCharacter.GlitchIntensity` 0 _asbp_first_person_character))

(fn `UserConstructionScript`)

(fn `VisionwireNaming`
  (returns (Name :type String) (IsMonster :type Boolean))
  (`self.Seen by Player`)
  (return "" false))