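; Door actor that swings open once when interacted with and can slam shut once.
; Opening plays a 2D sound while a timeline drives DoorLow's relative yaw from StartRotation by a scaled Rotation offset.
; SlamClose sets the yaw directly from a second timeline's track, then plays a close sound at the actor's location.
; VisionwireNaming reports the door as non-monster "DOOR" and triggers SlamClose as a side effect.
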(event `self.InteractedWith`
  (`/Engine/EditorBlueprintResources/StandardMacros.DoOnce` false
    (:`Completed`
      (`GameplayStatics.PlaySound2D` "/Game/_Content/_Audio/SC_Door.SC_Door" 1.0 1.0 0.0 null null)
      (bind (_direction _doortrack) (`Timeline|DoorTimeline`)
        (:`Update`
          (`SceneComponent.K2_SetRelativeRotation` (`self.Door_Low`) (`KismetMathLibrary.MakeRotator` 0.0 0.0 (+ (`self.StartRotation`) (* _doortrack (`self.Rotation`)))) false false))))))

(event `Slam Close`
  (`/Engine/EditorBlueprintResources/StandardMacros.DoOnce` false
    (:`Completed`
      (bind (_direction _doortrack) (`Timeline|Timeline`)
        (:`Update`
          (`SceneComponent.K2_SetRelativeRotation` (`self.Door_Low`) (`KismetMathLibrary.MakeRotator` 0.0 0.0 _doortrack) false false))
        (:`Finished`
          (`GameplayStatics.PlaySoundAtLocation` "/Game/_Content/_Audio/Door/Door_Close.Door_Close" (`self.K2_GetActorLocation`) (struct) 1.0 1.0 0.0 null null null null))))))

(fn `UserConstructionScript`)

(fn `VisionwireNaming`
  (returns (Name :type String) (IsMonster :type Boolean))
  (`self.Slam Close`)
  (return "DOOR" false))