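; BP_DoorStatic is an interactable door actor that turns into a solid wall the first time the player interacts with it.
; A DoOnce on the interaction event shows the wall mesh, hides the doorway and door meshes, and briefly spikes the first-person character's GlitchIntensity to mask or accent the swap.
; It reports its name to VisionwireNaming as a non-monster, then clears that name after the glitch ends.
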(event `/Game/_Content/_Blueprints/BPI_Interact.InteractedWith`
  (`/Engine/EditorBlueprintResources/StandardMacros.DoOnce` false
    (:`Completed`
      (bind _asbp_first_person_character (cast `/Game/FirstPerson/Blueprints/BP_FirstPersonCharacter` (`GameplayStatics.GetPlayerPawn` 0)))
      (`SceneComponent.SetVisibility` (`self.Wall_1`) true false)
      (`SceneComponent.SetVisibility` (`self.Wall_Doorway`) false false)
      (`SceneComponent.SetVisibility` (`self.Door_Low`) false false)
      (set `/Game/FirstPerson/Blueprints/BP_FirstPersonCharacter.GlitchIntensity` 2 _asbp_first_person_character)
      (`KismetSystemLibrary.Delay` 0.2)
      (set `/Game/FirstPerson/Blueprints/BP_FirstPersonCharacter.GlitchIntensity` 0 _asbp_first_person_character)
      (set `self.Name` ""))))

(fn `UserConstructionScript`)

(fn `VisionwireNaming`
  (returns (Name :type String) (IsMonster :type Boolean))
  (return (`self.Name`) false))