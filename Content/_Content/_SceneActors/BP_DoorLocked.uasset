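; BP_DoorLocked is a locked door scene actor that plays a locked-door 2D sound on interaction and never opens.
; Every Tick rolls a 1-in-5000 chance to play a knocking sound at the door, so knock frequency depends on frame rate.
; VisionwireNaming identifies it as a non-monster "DOOR".
; A timeline-driven swing-open rotation remains in the graph but is disconnected and never runs.
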(event `self.ReceiveTick`
  (params (DeltaSeconds :type "Float (single-precision)"))
  (`self.TriggerKnocking`))

(event `TriggerKnocking`
  (if (== (`KismetMathLibrary.RandomIntegerInRange` 1 5000) 1)
    (`GameplayStatics.PlaySoundAtLocation` "/Game/_Content/_Audio/SC_Knocking.SC_Knocking" (`self.K2_GetActorLocation`) (struct) 1.0 1.0 0.0 null null null null)))

(event `self.InteractedWith`
  (`GameplayStatics.PlaySound2D` "/Game/_Content/_Audio/SC_LockedDoor.SC_LockedDoor" 1.0 1.0 0.0 null null))

(fn `UserConstructionScript`)

(fn `VisionwireNaming`
  (returns (Name :type String) (IsMonster :type Boolean))
  (return "DOOR" false))