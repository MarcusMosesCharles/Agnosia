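; End-of-game door actor that swings open and closes out the sequence when its box trigger is first overlapped.
; The overlap plays a door sound and a timeline that yaws the door mesh from its start rotation.
; The first timeline update fires a one-shot End event that destroys the doppelganger, fades camera and audio to white, and removes all widgets.
; It reports itself as a non-monster "DOOR" through VisionwireNaming.
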(event `self.Box.OnComponentBeginOverlap`
  (params (OverlappedComponent :type "PrimitiveComponent Object Reference") (OtherActor :type "Actor Object Reference") (OtherComp :type "PrimitiveComponent Object Reference") (OtherBodyIndex :type Integer) (bFromSweep :type Boolean) (SweepResult :type "HitResult Structure (by ref)"))
  (`/Engine/EditorBlueprintResources/StandardMacros.DoOnce` false
    (:`Completed`
      (`GameplayStatics.PlaySound2D` "/Game/_Content/_Audio/SC_Door.SC_Door" 1.0 1.0 0.0 null null)
      (bind (_direction _doortrack) (`Timeline|DoorTimeline`)
        (:`Update`
          (`SceneComponent.K2_SetRelativeRotation` (`self.Door_Low`) (`KismetMathLibrary.MakeRotator` 0.0 0.0 (+ (`self.StartRotation`) (* _doortrack (`self.Rotation`)))) false false)
          (`self.End`))))))

(event `End`
  (`/Engine/EditorBlueprintResources/StandardMacros.DoOnce` false
    (:`Completed`
      (bind _returnvalue (`GameplayStatics.GetActorOfClass` "/Game/_Content/_Characters/Doppleganger/BPC_DoppleGanger.BPC_DoppleGanger_C"))
      (`self.K2_DestroyActor` _returnvalue)
      (`GameplayStatics.GetActorOfClass` "/Game/_Content/_SceneActors/BP_AmbientHumm.BP_AmbientHumm_C")
      (`PlayerCameraManager.StartCameraFade` (`GameplayStatics.GetPlayerCameraManager` 0) 0.0 1.0 5.0 (struct :`R` 1.0 :`G` 1.0 :`B` 1.0 :`A` 1.0) true true)
      (`WidgetLayoutLibrary.RemoveAllWidgets`))))

(fn `UserConstructionScript`)

(fn `VisionwireNaming`
  (returns (Name :type String) (IsMonster :type Boolean))
  (return "DOOR" false))