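; Light fixture actor that changes its look while a BPC_DoppleGanger is inside its Sphere trigger, apparently to flicker when that character is near.
; On begin overlap, it gives the RectLight a flicker light function material and swaps the Cube002 mesh to an alternate roof-item material.
; On end overlap, it sets the light function to WorldNormal and the mesh back to M_RoofItems, with no Tick or timers involved.
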(event `self.Sphere.OnComponentBeginOverlap`
  (params (OverlappedComponent :type "PrimitiveComponent Object Reference") (OtherActor :type "Actor Object Reference") (OtherComp :type "PrimitiveComponent Object Reference") (OtherBodyIndex :type Integer) (bFromSweep :type Boolean) (SweepResult :type "HitResult Structure (by ref)"))
  (cast `/Game/_Content/_Characters/Doppleganger/BPC_DoppleGanger` OtherActor)
  (`LightComponent.SetLightFunctionMaterial` (`self.RectLight`) "/Game/_Content/_StaticMeshes/Light/MI_Lightflicker_2.MI_Lightflicker_2")
  (`PrimitiveComponent.SetMaterial` (`self.Cube_002`) 0 "/Game/_Content/_StaticMeshes/RoofGround/Textures/M_RoofItems_2.M_RoofItems_2"))

(event `self.Sphere.OnComponentEndOverlap`
  (params (OverlappedComponent :type "PrimitiveComponent Object Reference") (OtherActor :type "Actor Object Reference") (OtherComp :type "PrimitiveComponent Object Reference") (OtherBodyIndex :type Integer))
  (cast `/Game/_Content/_Characters/Doppleganger/BPC_DoppleGanger` OtherActor)
  (`LightComponent.SetLightFunctionMaterial` (`self.RectLight`) "/Engine/BufferVisualization/WorldNormal.WorldNormal")
  (`PrimitiveComponent.SetMaterial` (`self.Cube_002`) 0 "/Game/_Content/_StaticMeshes/RoofGround/Textures/M_RoofItems.M_RoofItems"))

(fn `UserConstructionScript`)