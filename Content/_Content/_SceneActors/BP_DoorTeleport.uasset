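; BP_DoorTeleport is an interactable door that moves the player to a different height in the level, once only.
; Interaction passes a DoOnce, plays a door sound and briefly raises GlitchIntensity on the first-person character.
; After resetting the glitch, it teleports the player pawn to a hard-coded Z, keeping X and Y.
; VisionwireNaming identifies it as a non-monster named "DOOR".
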(event `self.InteractedWith`
  (bind _returnvalue (`GameplayStatics.GetPlayerPawn` 0))
  (bind (_returnvalue_x _returnvalue_y) (`KismetMathLibrary.BreakVector` (`self.K2_GetActorLocation` _returnvalue)))
  (`/Engine/EditorBlueprintResources/StandardMacros.DoOnce` false
    (:`Completed`
      (`GameplayStatics.PlaySound2D` "/Game/_Content/_Audio/SC_Door.SC_Door" 1.0 1.0 0.0 null null)
      (bind _asbp_first_person_character (cast `/Game/FirstPerson/Blueprints/BP_FirstPersonCharacter` _returnvalue))
      (set `/Game/FirstPerson/Blueprints/BP_FirstPersonCharacter.GlitchIntensity` 2 _asbp_first_person_character)
      (`KismetSystemLibrary.Delay` 0.2)
      (set `/Game/FirstPerson/Blueprints/BP_FirstPersonCharacter.GlitchIntensity` 0 _asbp_first_person_character)
      (`self.K2_SetActorLocation` _returnvalue (`KismetMathLibrary.MakeVector` _returnvalue_x _returnvalue_y 9081.0) false true))))

(fn `UserConstructionScript`)

(fn `VisionwireNaming`
  (returns (Name :type String) (IsMonster :type Boolean))
  (return "DOOR" false))